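; BP_Lou_SkillQ is the short-lived hit actor for Lou's Q skill, destroying itself one second after BeginPlay.
; A capsule hit spawns the NP_Lou_Hit Niagara effect and destroys the actor.
; An overlap spawns that effect only if a Character's capsule component is overlapping, then a DoOnce prints a damage placeholder and destroys the actor.
; No damage is applied yet.
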(event `self.Capsule.OnComponentHit`
  (params (HitComponent :type "PrimitiveComponent Object Reference") (OtherActor :type "Actor Object Reference") (OtherComp :type "PrimitiveComponent Object Reference") (NormalImpulse :type "Vector Structure") (Hit :type "HitResult Structure (by ref)"))
  ;[1 1 1] Component Hit
  (`NiagaraFunctionLibrary.SpawnSystemAtLocation` "/Game/__OWNER/Woong/FX/NP_Lou_Hit.NP_Lou_Hit" (`self.K2_GetActorLocation`))
  (`self.K2_DestroyActor`))

(event `self.ReceiveBeginPlay`
  ;[1 1 1] BeginPlay
  (`KismetSystemLibrary.Delay` 1.0)
  (`self.K2_DestroyActor`))

(event `self.Capsule.OnComponentBeginOverlap`
  (params (OverlappedComponent :type "PrimitiveComponent Object Reference") (OtherActor :type "Actor Object Reference") (OtherComp :type "PrimitiveComponent Object Reference") (OtherBodyIndex :type Integer) (bFromSweep :type Boolean) (SweepResult :type "HitResult Structure (by ref)"))
  ;[1 1 1] BeginOverlap
  ;[1 0 0.842] 액터가 오버랩된 것이 캐릭터의 캡슐 컴포넌트라면 실행
  (bind _ascharacter (cast `Character` OtherActor))
  (if (`PrimitiveComponent.IsOverlappingComponent` (`Character.CapsuleComponent` _ascharacter) (`self.Capsule`))
    (`NiagaraFunctionLibrary.SpawnSystemAtLocation` "/Game/__OWNER/Woong/FX/NP_Lou_Hit.NP_Lou_Hit" (`self.K2_GetActorLocation`))
    (`/Engine/EditorBlueprintResources/StandardMacros.DoOnce` false
      (:`Completed`
        (`KismetSystemLibrary.PrintString` "Damage 로직" true true (struct :`R` 0.287343 :`G` 1.0 :`A` 1.0))
        (`self.K2_DestroyActor`)))))

(fn `UserConstructionScript`)