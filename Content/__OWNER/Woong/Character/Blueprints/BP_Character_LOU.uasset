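; Player character Blueprint for Lou, handling cursor-aimed Q and W skills.
; Tick keeps CursorToWorld under the mouse, and each cast turns the actor toward it before spawning from SkillArrowPoint.
; Q fires twice with a short delay; W saves the cursor point and is blocked while its projectile or blizzard effect exists.
; When the W actor nears that point, Tick replaces it with blizzard and ground Niagara effects plus a ground collision actor.
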(event `Key|W`
  (params (Key :type "Key Structure"))
  ;[1 1 1] W Skill
  (:`Pressed`
    ;[1 1 1] W 사용 시, 공격이 끝날 때까지 사용 금지
    (`/Engine/EditorBlueprintResources/StandardMacros.IsValid` (`self.SkillW`)
      (:`Is Not Valid`
        (`/Engine/EditorBlueprintResources/StandardMacros.IsValid` (`self.NPSkillW_Blizzard`)
          (:`Is Not Valid`
            ;[0.8052 0.328 0.328] 스킬 W 발동 시, 마우스 포인터 위치 저장
            (`self.EventSpawnSkillB`)
            (`self.FindActorToMouseRotation`)
            (`self.TurnActor`)
            (bind _spawnactorvalue (`self.SpawnSkill_ReturnValuePlus` (`self.BPSkillW`) (`self.SkillArrowPoint`)))
            (set `self.SkillW` _spawnactorvalue)))))))

(event `SpawnSkillW_NP`
  ;[0.301 0.01976 0.01976] W 소멸 되었을 때 실행
  ;[1 1 1] Lou Skill W 나이아가라 파티클 생성
  (bind _returnvalue (`NiagaraFunctionLibrary.SpawnSystemAtLocation` "/Game/__OWNER/Woong/FX/NP_LouSkillW_Blizzard.NP_LouSkillW_Blizzard" (`self.SaveNPSpawnPoint`)))
  (set `self.NPSkillW_Blizzard` _returnvalue)
  (bind _returnvalue_2 (`NiagaraFunctionLibrary.SpawnSystemAtLocation` "/Game/__OWNER/Woong/FX/NP_LouSkillW_Ground.NP_LouSkillW_Ground" (`self.SaveNPSpawnPoint`)))
  (set `self.NPSkillW_Gournd` _returnvalue_2)
  ;[1 1 1] Lou Skill W 범위 콜리전 생성
  (`|SpawnActorFromClass` "/Game/__OWNER/Woong/Blueprints/BP_Lou_SkillW_Ground.BP_Lou_SkillW_Ground_C" (`KismetMathLibrary.MakeTransform` (`self.SaveNPSpawnPoint`)) "Undefined" "OverrideRootScale" null null))

(event `self.ReceiveTick`
  (params (DeltaSeconds :type "Float (single-precision)"))
  (bind _skillw (`self.SkillW`))
  (bind _returnvalue (`self.K2_GetActorLocation` _skillw))
  (bind (_bblockinghit _binitialoverlap _time _distance _location _impactpoint _normal _impactnormal) (`GameplayStatics.BreakHitResult` (`PlayerController.GetHitResultUnderCursorByChannel` (`GameplayStatics.GetPlayerController` 0) "TraceTypeQuery1" true)))
  ;[1 1 1] Tick
  (`|ExecutionSequence`
    (:`then_0`
      ;[1 1 1] W 활성화 시, 실행
      (`/Engine/EditorBlueprintResources/StandardMacros.IsValid` _skillw
        (:`Is Valid`
          (if (== _returnvalue (`self.SaveNPSpawnPoint`) :`ErrorTolerance` 80.0)
            (set `self.SaveNPSpawnPoint` _returnvalue)
            ;[0.301 0.01976 0.01976] W 소멸 되었을 때 실행
            (`self.SpawnSkillW_NP`)
            (`self.K2_DestroyActor` (`self.SkillW`))))))
    (:`then_1`
      ;[1 1 1] 매 프레임 커서의 트랜스폼을 설정
      (`SceneComponent.K2_SetWorldLocationAndRotation` (`self.CursorToWorld`) _location (`KismetMathLibrary.MakeRotationFromAxes` _impactnormal) false false))))

(event `Key|Q`
  (params (Key :type "Key Structure"))
  ;[1 1 1] Q Skill
  (:`Pressed`
    ;[1 1 1] 액터와 마우스 사이의 회전값 저장
    (`self.FindActorToMouseRotation`)
    ;[1 1 1] 액터를 마우스 포인터의 방향으로 턴
    (`self.TurnActor`)
    ;[1 1 1] 액터 스폰
    (`self.SpawnSkill` (`self.BPSkillQ`) (`self.SkillArrowPoint`))
    ;[1 1 1] 한번 더 실행
    (`KismetSystemLibrary.Delay` 0.15)
    (`self.TurnActor`)
    (`self.SpawnSkill` (`self.BPSkillQ`) (`self.SkillArrowPoint`))))

(event `EventSpawnSkillB`
  ;[0.8052 0.328 0.328] 스킬 W 발동 시, 마우스 포인터 위치 저장
  (set `self.SaveNPSpawnPoint` (`.Location` (`GameplayStatics.BreakHitResult` (`PlayerController.GetHitResultUnderCursorByChannel` (`GameplayStatics.GetPlayerController` 0) "TraceTypeQuery1" true)))))

(fn `FindActorToMouseRotation`
  (bind (_returnvalue_x _returnvalue_y _returnvalue_z) (`KismetMathLibrary.BreakVector` (`self.K2_GetActorLocation`)))
  (bind (_returnvalue_x_2 _returnvalue_y_2) (`KismetMathLibrary.BreakVector` (`SceneComponent.K2_GetComponentLocation` (`self.CursorToWorld`))))
  ;[1 1 1 0] 액터와 마우스 사이의 회전값 저장
  (set `self.FindRotation` (`KismetMathLibrary.FindLookAtRotation` (`KismetMathLibrary.MakeVector` _returnvalue_x _returnvalue_y _returnvalue_z) (`KismetMathLibrary.MakeVector` _returnvalue_x_2 _returnvalue_y_2 _returnvalue_z))))

(fn `SpawnNP`
  (params (SpawnLocation :type "Vector Structure"))
  (returns (SpawnNP_Value :type "NiagaraComponent Object Reference"))
  (bind _returnvalue (`NiagaraFunctionLibrary.SpawnSystemAtLocation` "/Game/__OWNER/Woong/FX/NP_LouSkillW_Ground.NP_LouSkillW_Ground" SpawnLocation))
  (bind _output_get (set `self.NPSkillW_Gournd` _returnvalue))
  (return _output_get))

(fn `SpawnSkill`
  (params (SpawnSkillClass :type "Actor Class Reference") (GetWorldLocationTarget :type "SceneComponent Object Reference"))
  (bind (_returnvalue_location _returnvalue_rotation _returnvalue_scale) (`KismetMathLibrary.BreakTransform` (`self.GetTransform`)))
  ;[1 1 1 0] 액터 스폰
  (`|SpawnActorFromClass` SpawnSkillClass (`KismetMathLibrary.MakeTransform` (`SceneComponent.K2_GetComponentLocation` GetWorldLocationTarget) _returnvalue_rotation _returnvalue_scale) "Undefined" "OverrideRootScale" null null))

(fn `SpawnSkill_ReturnValuePlus`
  (params (SpawnSkillClass :type "Actor Class Reference") (GetWorldLocationTarget :type "SceneComponent Object Reference"))
  (returns (SpawnActorValue :type "Actor Object Reference"))
  (bind (_returnvalue_location _returnvalue_rotation _returnvalue_scale) (`KismetMathLibrary.BreakTransform` (`self.GetTransform`)))
  ;[1 1 1 0] 액터 스폰
  (bind _returnvalue (`|SpawnActorFromClass` SpawnSkillClass (`KismetMathLibrary.MakeTransform` (`SceneComponent.K2_GetComponentLocation` GetWorldLocationTarget) _returnvalue_rotation _returnvalue_scale) "Undefined" "OverrideRootScale" self null))
  (return _returnvalue))

(fn `TurnActor`
  ;[1 1 1 0] 액터를 마우스 포인터의 방향으로 턴
  (`self.K2_SetActorRelativeRotation` (`self.FindRotation`)))

(fn `UserConstructionScript`)