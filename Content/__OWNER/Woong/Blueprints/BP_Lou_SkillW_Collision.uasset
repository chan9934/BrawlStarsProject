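; Short-lived sphere area for Lou's W skill that puts a status effect on characters inside it and destroys itself after a fixed delay.
; Capsule overlap with the sphere sets the third PlayerStateManager flag, preserving bleeding and toxic flags; leaving clears it.
; Each hero class (Amber, Lou, Edgar, Max) is handled by a cast chain.
; The owner is excluded only when setting the flag, not when clearing it.
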(event `self.ReceiveBeginPlay`
  ;[1 1 1] BeginPlay
  (`KismetSystemLibrary.Delay` 5.4)
  (`self.K2_DestroyActor`))

(event `self.Sphere.OnComponentBeginOverlap`
  (params (OverlappedComponent :type "PrimitiveComponent Object Reference") (OtherActor :type "Actor Object Reference") (OtherComp :type "PrimitiveComponent Object Reference") (OtherBodyIndex :type Integer) (bFromSweep :type Boolean) (SweepResult :type "HitResult Structure (by ref)"))
  ;[1 1 1] BeginOverlap
  (bind _ascharacter (cast `Character` OtherActor))
  (if (`PrimitiveComponent.IsOverlappingComponent` (`Character.CapsuleComponent` _ascharacter) (`self.Sphere`))
    (set `self.EnemyActor` _ascharacter)
    (if (not (== (`self.EnemyActor`) (`self.GetOwner`)))
      (bind _asamber_bp (cast `/Game/__OWNER/Rudals/Blueprints/Amber_BP` (`self.EnemyActor`))
        (:`then`
          (bind (_playerstatemanager_bisblooding _playerstatemanager_bistoxicating) (break `S_PlayerState` (`/Game/__OWNER/Rudals/Blueprints/Amber_BP.PlayerStateManager` _asamber_bp)))
          (set `/Game/__OWNER/Rudals/Blueprints/Amber_BP.PlayerStateManager` (make `S_PlayerState` _playerstatemanager_bisblooding _playerstatemanager_bistoxicating true) _asamber_bp))
        (:`CastFailed`
          (bind _asbp_character_lou (cast `/Game/__OWNER/Woong/Character/Blueprints/BP_Character_LOU` (`self.EnemyActor`))
            (:`then`
              (bind (_playerstatemanager_bisblooding_2 _playerstatemanager_bistoxicating_2) (break `S_PlayerState` (`/Game/__OWNER/Woong/Character/Blueprints/BP_Character_LOU.PlayerStateManager` _asbp_character_lou)))
              (set `/Game/__OWNER/Woong/Character/Blueprints/BP_Character_LOU.PlayerStateManager` (make `S_PlayerState` _playerstatemanager_bisblooding_2 _playerstatemanager_bistoxicating_2 true) _asbp_character_lou))
            (:`CastFailed`
              (bind _asbp_edgar (cast `/Game/__OWNER/DongChan/Blueprint/BP_Edgar` (`self.EnemyActor`))
                (:`then`
                  (bind (_playerstatemanager_bisblooding_3 _playerstatemanager_bistoxicating_3) (break `S_PlayerState` (`/Game/__OWNER/DongChan/Blueprint/BP_Edgar.PlayerStateManager` _asbp_edgar)))
                  (set `/Game/__OWNER/DongChan/Blueprint/BP_Edgar.PlayerStateManager` (make `S_PlayerState` _playerstatemanager_bisblooding_3 _playerstatemanager_bistoxicating_3 true) _asbp_edgar))
                (:`CastFailed`
                  (bind _asbp_max (cast `/Game/__OWNER/SYL/Character/BP_Max` (`self.EnemyActor`)))
                  (bind (_playerstatemanager_bisblooding_4 _playerstatemanager_bistoxicating_4) (break `S_PlayerState` (`/Game/__OWNER/SYL/Character/BP_Max.PlayerStateManager` _asbp_max)))
                  (set `/Game/__OWNER/SYL/Character/BP_Max.PlayerStateManager` (make `S_PlayerState` _playerstatemanager_bisblooding_4 _playerstatemanager_bistoxicating_4 true) _asbp_max))))))))))

(event `self.Sphere.OnComponentEndOverlap`
  (params (OverlappedComponent :type "PrimitiveComponent Object Reference") (OtherActor :type "Actor Object Reference") (OtherComp :type "PrimitiveComponent Object Reference") (OtherBodyIndex :type Integer))
  ;[1 1 1] EndOverlap
  (bind _ascharacter (cast `Character` OtherActor))
  (if (not (`PrimitiveComponent.IsOverlappingComponent` (`Character.CapsuleComponent` _ascharacter) (`self.Sphere`)))
    (set `self.EnemyActor` _ascharacter)
    (bind _asamber_bp (cast `/Game/__OWNER/Rudals/Blueprints/Amber_BP` (`self.EnemyActor`))
      (:`then`
        (bind (_playerstatemanager_bisblooding _playerstatemanager_bistoxicating) (break `S_PlayerState` (`/Game/__OWNER/Rudals/Blueprints/Amber_BP.PlayerStateManager` _asamber_bp)))
        (set `/Game/__OWNER/Rudals/Blueprints/Amber_BP.PlayerStateManager` (make `S_PlayerState` _playerstatemanager_bisblooding _playerstatemanager_bistoxicating) _asamber_bp))
      (:`CastFailed`
        (bind _asbp_character_lou (cast `/Game/__OWNER/Woong/Character/Blueprints/BP_Character_LOU` (`self.EnemyActor`))
          (:`then`
            (bind (_playerstatemanager_bisblooding_2 _playerstatemanager_bistoxicating_2) (break `S_PlayerState` (`/Game/__OWNER/Woong/Character/Blueprints/BP_Character_LOU.PlayerStateManager` _asbp_character_lou)))
            (set `/Game/__OWNER/Woong/Character/Blueprints/BP_Character_LOU.PlayerStateManager` (make `S_PlayerState` _playerstatemanager_bisblooding_2 _playerstatemanager_bistoxicating_2) _asbp_character_lou))
          (:`CastFailed`
            (bind _asbp_edgar (cast `/Game/__OWNER/DongChan/Blueprint/BP_Edgar` (`self.EnemyActor`))
              (:`then`
                (bind (_playerstatemanager_bisblooding_3 _playerstatemanager_bistoxicating_3) (break `S_PlayerState` (`/Game/__OWNER/DongChan/Blueprint/BP_Edgar.PlayerStateManager` _asbp_edgar)))
                (set `/Game/__OWNER/DongChan/Blueprint/BP_Edgar.PlayerStateManager` (make `S_PlayerState` _playerstatemanager_bisblooding_3 _playerstatemanager_bistoxicating_3) _asbp_edgar))
              (:`CastFailed`
                (bind _asbp_max (cast `/Game/__OWNER/SYL/Character/BP_Max` (`self.EnemyActor`)))
                (bind (_playerstatemanager_bisblooding_4 _playerstatemanager_bistoxicating_4) (break `S_PlayerState` (`/Game/__OWNER/SYL/Character/BP_Max.PlayerStateManager` _asbp_max)))
                (set `/Game/__OWNER/SYL/Character/BP_Max.PlayerStateManager` (make `S_PlayerState` _playerstatemanager_bisblooding_4 _playerstatemanager_bistoxicating_4) _asbp_max)))))))))

(fn `UserConstructionScript`)