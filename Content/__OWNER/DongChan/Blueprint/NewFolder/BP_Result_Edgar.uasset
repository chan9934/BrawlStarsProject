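; BP_Result_Edgar is a display actor for the Edgar character, apparently for a match result screen.
; On BeginPlay it passes its BrawlScroe value to the Score of its Umg_First widget component.
; It then plays a one-shot lobby animation chosen by world position: Edgar_Lobby_Rev3 when Y is near zero, otherwise the Not_Effect variant.
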(event `self.ReceiveTick`
  (params (DeltaSeconds :type "Float (single-precision)")))

(event `SetUi`
  (bind _asumg_first (cast `/Game/__OWNER/DongChan/UMG/Umg_First` (`WidgetComponent.GetWidget` (`self.Widget`))))
  (set `/Game/__OWNER/DongChan/UMG/Umg_First.Score` (`self.BrawlScroe`) _asumg_first))

(event `self.ReceiveBeginPlay`
  (bind (_returnvalue_x _returnvalue_y) (`KismetMathLibrary.BreakVector` (`self.K2_GetActorLocation`)))
  (bind _skeletalmesh1 (`self.SkeletalMesh1`))
  (`self.SetUi`)
  (if (`KismetMathLibrary.InRange_FloatFloat` _returnvalue_y -10.0 10.0)
    (`SkeletalMeshComponent.PlayAnimation` _skeletalmesh1 "/Game/__OWNER/DongChan/edgar/NewAnim/Edgar_Lobby_Rev3.Edgar_Lobby_Rev3" false)
    (else
      (`SkeletalMeshComponent.PlayAnimation` _skeletalmesh1 "/Game/__OWNER/DongChan/edgar/NewAnim/Edgar_Lobby_Not_Effect.Edgar_Lobby_Not_Effect" false))))

(fn `UserConstructionScript`)