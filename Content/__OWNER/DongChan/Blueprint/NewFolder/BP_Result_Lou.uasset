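; BP_Result_Lou is an actor that presents the Lou character with a score widget, apparently for a result screen.
; On BeginPlay it passes BrawlScore into the Umg_First widget held by its Widget component.
; It then plays a one-shot lobby animation on the skeletal mesh, choosing the version with effects only when the actor sits near zero on world Y, otherwise the no-effect version.
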(event `self.ReceiveBeginPlay`
  (bind (_returnvalue_x _returnvalue_y) (`KismetMathLibrary.BreakVector` (`self.K2_GetActorLocation`)))
  (bind _skeletalmesh (`self.SkeletalMesh`))
  (bind _asumg_first (cast `/Game/__OWNER/DongChan/UMG/Umg_First` (`WidgetComponent.GetWidget` (`self.Widget`))))
  (set `/Game/__OWNER/DongChan/UMG/Umg_First.Score` (`self.BrawlScore`) _asumg_first)
  (if (`KismetMathLibrary.InRange_FloatFloat` _returnvalue_y -10.0 10.0)
    (`SkeletalMeshComponent.PlayAnimation` _skeletalmesh "/Game/__OWNER/DongChan/LouAnim/Lobby_Lou.Lobby_Lou" false)
    (else
      (`SkeletalMeshComponent.PlayAnimation` _skeletalmesh "/Game/__OWNER/DongChan/LouAnim/Lobby_Lou_No_Effect.Lobby_Lou_No_Effect" false))))

(fn `UserConstructionScript`)